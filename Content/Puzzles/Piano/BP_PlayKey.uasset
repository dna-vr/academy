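; VR piano puzzle key that glows and plays its note sequence when a MotionControllerPawn overlaps its box.
; A looping timer plays and removes the first Note entry each step, then restores the array from Backup once empty.
; A Timeline drives the Glow parameter on the key's dynamic material.
; Tick prints solved or awaiting status, based on notes having played and Note matching CorrectCombo.
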(event OnComponentBeginOverlap(Box)
  (params (OverlappedComponent :type Primitive%20Component%20Object%20Reference) (OtherActor :type Actor%20Object%20Reference) (OtherComp :type Primitive%20Component%20Object%20Reference) (OtherBodyIndex :type Integer) (bFromSweep :type Boolean) (SweepResult :type Hit%20Result%20Structure%20%28by%20ref%29))
  (Utilities|Casting|CastToMotionControllerPawn OtherActor)
  (Utilities|FlowControl|Sequence
    (:then_0
      (Variables|Default|SetBackup (Variables|Default|GetNote))
      (bind _returnvalue (Utilities|Time|SetTimerbyEvent (delegate Custom|Play%20Notes) 0.3 true)))
    (:then_1
      (bind _newtrack_0 (Timeline|Timeline_0 PlayFromStart)
        (:Update
          (Rendering|Material|SetScalarParameterValue (stale EventBeginPlay _returnvalue) "Glow" _newtrack_0 :!class /Script/Engine.MaterialInstanceDynamic))))))

(event Custom|Play%20Notes
  (Audio|PlaySound2D (Utilities|Array|Get(acopy) (Variables|Default|GetNote)) 1.0 1.0 0.0 0 0)
  (Variables|Default|SetNotes%20Played true)
  (Utilities|Array|RemoveIndex (Variables|Default|GetNote))
  (Utilities|IsValid (Utilities|Array|Get(acopy) (Variables|Default|GetNote))
    (:Is%20Not%20Valid
      (Utilities|Time|ClearandInvalidateTimerbyHandle (stale OnComponentBeginOverlap(Box) _returnvalue))
      (Variables|Default|SetNote (Variables|Default|GetBackup)))))

(event EventBeginPlay
  (bind _key_mesh (Variables|Default|GetKey_Mesh))
  (bind _returnvalue (Rendering|Material|CreateDynamicMaterialInstance _key_mesh 0 0 "None" :!class /Script/Engine.PrimitiveComponent))
  (Rendering|Material|SetMaterial _key_mesh 0 _returnvalue))

(event EventTick
  (params (DeltaSeconds :type Float%20%28single-precision%29))
  ;[0.3345 1 0.4445] Check if true
  (if (and (Variables|Default|GetNotes%20Played) (Utilities|Array|Identical (Variables|Default|GetCorrectCombo) (Variables|Default|GetNote)))
    (Development|PrintString "Piano Solved" true true "(R=0.229378,G=0.880104,B=1.000000,A=1.000000)" 0.01)
    (else
      (Development|PrintString "Piano Awaiting" true true "(R=1.000000,G=0.908769,B=0.324843,A=1.000000)" 0.01))))

(fn ConstructionScript)