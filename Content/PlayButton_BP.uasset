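; A lyre puzzle play button that responds to motion controller touch and can open its owning sliding door.
; Overlap backs up the note array, starts a one-shot timer for PlayNotes and animates material glow through a timeline.
; PlayNotes plays and removes the first note, restoring the backup once none remain.
; Tick marks the owning BP_Door_Slide2 solved when NotesPlayed is true and the notes match the correct combo.
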(event OnComponentBeginOverlap(Capsule)
  (params (OverlappedComponent :type Primitive%20Component%20Object%20Reference) (OtherActor :type Actor%20Object%20Reference) (OtherComp :type Primitive%20Component%20Object%20Reference) (OtherBodyIndex :type Integer) (bFromSweep :type Boolean) (SweepResult :type Hit%20Result%20Structure%20%28by%20ref%29))
  (Utilities|Casting|CastToBP_MotionController OtherActor)
  (Utilities|FlowControl|Sequence
    (:then_0
      (Variables|Default|SetBackup_Note (Variables|Default|GetLyre_Note))
      (bind _returnvalue (Utilities|Time|SetTimerbyEvent (delegate Custom|Play%20Notes) 0.3)))
    (:then_1
      (bind _newtrack_2 (Timeline|Timeline_0 Play)
        (:Update
          (Rendering|Material|SetScalarParameterValue (stale EventBeginPlay _returnvalue) "Glow" _newtrack_2 :!class /Script/Engine.MaterialInstanceDynamic))))))

(event Custom|Play%20Notes
  (Audio|PlaySound2D (Utilities|Array|Get(acopy) (Variables|Default|GetLyre_Note)) 1.0 1.0 0.0 0 0)
  (Utilities|Array|RemoveIndex (Variables|Default|GetLyre_Note))
  (Utilities|IsValid (Utilities|Array|Get(acopy) (Variables|Default|GetLyre_Note))
    (:Is%20Not%20Valid
      (Utilities|Time|ClearandInvalidateTimerbyHandle (stale OnComponentBeginOverlap(Capsule) _returnvalue))
      (Variables|Default|SetLyre_Note (Variables|Default|GetBackup_Note)))))

(event EventBeginPlay
  (bind _staticmesh (Variables|Default|GetStaticMesh))
  (bind _returnvalue (Rendering|Material|CreateDynamicMaterialInstance _staticmesh 0 "/Game/LESSONS/Lyre/Assets/String_M.String_M" "None" :!class /Script/Engine.PrimitiveComponent))
  (Rendering|Material|SetMaterial _staticmesh 0 _returnvalue))

(event Collision|EventActorBeginOverlap
  (params (OtherActor :type Actor%20Object%20Reference)))

(event EventTick
  (params (DeltaSeconds :type Float%20%28single-precision%29))
  ;[1 1 1] Check if played combo matches correct combo & if play button has been hit
  (if (and (Variables|Default|GetNotes%20Played) (Utilities|Array|Identical (Variables|Default|GetCorrectCombo) (Variables|Default|GetLyre_Note)))
    ;[1 1 1] Open Door
    (bind _asbp_door_slide_2 (Utilities|Casting|CastToBP_Door_Slide2 (Components|GetOwner)))
    (Variables|/Game/GAME/Doors/BP_Door_Slide2.BP_Door_Slide2_C|SetPuzzleSolved _asbp_door_slide_2 true)))

(fn ConstructionScript)