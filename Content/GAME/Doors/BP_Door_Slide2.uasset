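; Double sliding door, "Door 3", that opens on a Door 3 opened event bound at BeginPlay and closes behind the player.
; The Open timeline drives the relative locations of both door panels, with a 2D slide sound on each move.
; A VR motion controller entering the Box trigger reverses the timeline through a DoOnce, closing the door a single time.
; Debug prints mark the opening and the player leaving.
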(event OnComponentBeginOverlap(Box)
  (params (OverlappedComponent :type Primitive%20Component%20Object%20Reference) (OtherActor :type Actor%20Object%20Reference) (OtherComp :type Primitive%20Component%20Object%20Reference) (OtherBodyIndex :type Integer) (bFromSweep :type Boolean) (SweepResult :type Hit%20Result%20Structure%20%28by%20ref%29))
  (Utilities|Casting|CastToBP_MotionController OtherActor)
  (Utilities|FlowControl|DoOnce false
    (:Completed
      (Utilities|FlowControl|Sequence
        (:then_0
          (bind (_direction _door_right _door_left _doorl _doorr) (Timeline|Open Reverse)
            (:Update
              (Utilities|FlowControl|Sequence
                (:then_0
                  (Transformation|SetRelativeLocation (Variables|Default|GetDoor_Left) _doorl false false))
                (:then_1
                  (Transformation|SetRelativeLocation (Variables|Default|GetDoor_Right) _doorr false false))))))
        (:then_1
          (Audio|PlaySound2D "/Game/LESSONS/KeyDoor/Assets/SFX/Door_Slide.Door_Slide" 1.0 1.0 0.0 0 0))
        (:then_2
          (Development|PrintString "Player Left"))))))

(event Custom|OpenDoor3
  (Development|PrintString "DOOR 3 OPENS")
  (Utilities|FlowControl|Sequence
    (:then_0
      (bind (_direction _door_right _door_left _doorl _doorr) (Timeline|Open Play)
        (:Update
          (Utilities|FlowControl|Sequence
            (:then_0
              (Transformation|SetRelativeLocation (Variables|Default|GetDoor_Left) _doorl false false))
            (:then_1
              (Transformation|SetRelativeLocation (Variables|Default|GetDoor_Right) _doorr false false))))))
    (:then_1
      (Audio|PlaySound2D "/Game/LESSONS/KeyDoor/Assets/SFX/Door_Slide.Door_Slide" 1.0 1.0 0.0 0 0))))

(event EventTick
  (params (DeltaSeconds :type Float%20%28single-precision%29)))

(event EventBeginPlay
  (EventDispatchers|BindEventtoDoor3Opened (delegate Custom|OpenDoor3)))

(fn ConstructionScript)