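; BP_Door_Slide1 is a double sliding door that responds to a BP_Key1 actor overlapping its Box trigger.
; Key entry plays the Open timeline, which drives both panels' relative locations, then plays a slide sound and destroys the key.
; Key exit reverses the timeline and reuses that sound-and-destroy chain.
; A MotionControllerPawn leaving the trigger unloads the Room2 streaming level.
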(event OnComponentBeginOverlap(Box)
  (params (OverlappedComponent :type Primitive%20Component%20Object%20Reference) (OtherActor :type Actor%20Object%20Reference) (OtherComp :type Primitive%20Component%20Object%20Reference) (OtherBodyIndex :type Integer) (bFromSweep :type Boolean) (SweepResult :type Hit%20Result%20Structure%20%28by%20ref%29))
  (Utilities|Casting|CastToBP_Key1 OtherActor)
  (Utilities|FlowControl|Sequence
    (:then_0
      (bind (_direction _door_right _door_left _doorl _doorr) (Timeline|Open Play)
        (:Update
          (Utilities|FlowControl|Sequence
            (:then_0
              (Transformation|SetRelativeLocation (Variables|Default|GetDoor_Left) _doorl false false))
            (:then_1
              (Transformation|SetRelativeLocation (Variables|Default|GetDoor_Right) _doorr false false))))))
    (:then_1
      (Audio|PlaySound2D "/Game/LESSONS/KeyDoor/Assets/SFX/Door_Slide.Door_Slide" 1.0 1.0 0.0 0 0)
      (Actor|DestroyActor (stale OnComponentEndOverlap(Box) _asbp_key_1)))))

(event OnComponentEndOverlap(Box)
  (params (OverlappedComponent :type Primitive%20Component%20Object%20Reference) (OtherActor :type Actor%20Object%20Reference) (OtherComp :type Primitive%20Component%20Object%20Reference) (OtherBodyIndex :type Integer))
  (Utilities|FlowControl|Sequence
    (:then_0
      (bind _asbp_key_1 (Utilities|Casting|CastToBP_Key1 OtherActor))
      (Utilities|FlowControl|Sequence
        (:then_0
          (Development|PrintString "Key Left")
          (bind (_direction _door_right _door_left _doorl _doorr) (Timeline|Open Reverse)
            (:Update
              (Utilities|FlowControl|Sequence
                (:then_0
                  (Transformation|SetRelativeLocation (Variables|Default|GetDoor_Left) _doorl false false))
                (:then_1
                  (Transformation|SetRelativeLocation (Variables|Default|GetDoor_Right) _doorr false false))))))
        (:then_1
          (Audio|PlaySound2D "/Game/LESSONS/KeyDoor/Assets/SFX/Door_Slide.Door_Slide" 1.0 1.0 0.0 0 0)
          (Actor|DestroyActor _asbp_key_1))))
    (:then_1
      (Utilities|Casting|CastToMotionControllerPawn OtherActor)
      (Game|UnloadStreamLevel(byName) "Room2" false))))

(fn ConstructionScript)