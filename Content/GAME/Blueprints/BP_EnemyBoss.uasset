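; Enemy boss that shoots at the player on sight and triggers the player's win when killed.
; Pawn sensing turns it toward the player and launches an impulse-driven BP_BossAttack, with a delay that both limits fire rate and destroys the projectile.
; BP_BulletFire hits on the capsule reduce health until it dies.
; Random patrol points are set up, but the timeline movement that would use them never runs.
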(event OnSeePawn(PawnSensing)
  (params (Pawn :type Pawn%20Object%20Reference))
  (bind _asmotion_controller_pawn (Utilities|Casting|CastToMotionControllerPawn Pawn))
  (Development|PrintString "PLAYER SPOTTED")
  (Utilities|FlowControl|Sequence
    (:then_0
      (Transformation|SetActorRotation (Math|Rotator|FindLookatRotation (Transformation|GetActorLocation) (Transformation|GetActorLocation _asmotion_controller_pawn))))
    (:then_1
      (if (Variables|Default|GetSpawnProjectile)
        (bind _returnvalue (Game|SpawnActorfromClass "/Game/LESSONS/BossFight/BP_BossAttack.BP_BossAttack_C" (Transformation|GetWorldTransform (Variables|Default|GetProjectileSpawnLocation)) "Undefined" 0 0))
        (Physics|AddImpulse (Variables|/Game/LESSONS/BossFight/BP_BossAttack.BP_BossAttack_C|GetSphere _returnvalue) (* (Math|Vector|GetForwardVector (Variables|Default|GetProjectileSpawnLocation)) (Variables|Default|GetShootForce)) "None" false)
        (Variables|Default|SetSpawnProjectile false)
        (Utilities|FlowControl|Delay 1.5)
        (Actor|DestroyActor _returnvalue)
        (Variables|Default|SetSpawnProjectile true)))))

(event OnComponentHit(CapsuleComponent)
  (params (HitComponent :type Primitive%20Component%20Object%20Reference) (OtherActor :type Actor%20Object%20Reference) (OtherComp :type Primitive%20Component%20Object%20Reference) (NormalImpulse :type Vector :default "0, 0, 0") (Hit :type Hit%20Result%20Structure%20%28by%20ref%29))
  (Utilities|Casting|CastToBP_BulletFire OtherActor)
  (Effects|SpawnEmitteratLocation "/Game/GAME/Other/FXVarietyPack/Particles/P_ky_hit1.P_ky_hit1" "0, 0, 0")
  (Variables|Default|SetHealth (- (Variables|Default|GetHealth) (Variables|Default|GetDamage)))
  (Development|PrintString "Enemy Health Decreased")
  (if (<= (Variables|Default|GetHealth) 0)
    (bind _asmotion_controller_pawn (Utilities|Casting|CastToMotionControllerPawn (Game|Player|GetPlayerPawn 0)))
    (Default|CallPlayerWon _asmotion_controller_pawn)
    (Development|PrintString "Alien Defeated")
    (Variables|Default|SetEscaped true)
    (Actor|DestroyActor)))

(event Collision|EventActorBeginOverlap
  (params (OtherActor :type Actor%20Object%20Reference)))

(event EventTick
  (params (DeltaSeconds :type Float%20%28single-precision%29)))

(event EventBeginPlay
  ;[1 1 1] SetPatrolPoints
  (Variables|Default|SetPatrolPoints (Utilities|Array|MakeArray (Transformation|GetWorldLocation (Variables|Default|GetMovePosition1)) (Transformation|GetWorldLocation (Variables|Default|GetMovePosition2)) (Transformation|GetWorldLocation (Variables|Default|GetMovePosition3))))
  (CallFunction|GetRandomLocation))

(fn ConstructionScript)

(fn GetRandomLocation
  (Variables|Default|SetCurrentPatrolPoint (Math|Random|RandomInteger (Utilities|Array|Length (Variables|Default|GetPatrolPoints)))))