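; Countdown is an actor that, despite its name, counts upward and shows minutes and seconds on two text displays.
; Each Tick increments the seconds, rolling into minutes after 59, with no delta-time scaling, so its speed follows the tick rate.
; RecordTime prints a congratulatory message with the final time and disables ticking to stop the clock.
; Leftover decrement logic is disconnected and never runs.
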(event Custom|RecordTime
  (bind _output_get (Variables|Default|SetTime (Utilities|String|BuildString(Integer) (Utilities|String|BuildString(Integer) "Congrats!" "Your time is:" (Variables|Default|GetMin) "minutes") "and" (Variables|Default|GetSec) "seconds")))
  (Development|PrintString _output_get)
  (Actor|Tick|SetActorTickEnabled false))

(event EventBeginPlay)

(event EventTick
  (params (DeltaSeconds :type Float%20%28single-precision%29))
  (if (== (Variables|Default|GetSec) 59)
    (Utilities|FlowControl|Sequence
      (:then_0
        (bind _output_get (Variables|Default|SetSec 0))
        (Rendering|Components|TextRender|SetText (Variables|Default|GetSeconds) (Utilities|Text|ToText(Integer) _output_get)))
      (:then_1
        (bind _result (Math|Integer|IncrementInt (Variables|Default|GetMin))
          (:%20%20
            (bind _output_get_2 (Variables|Default|SetMin _result))
            (Rendering|Components|TextRender|SetText (Variables|Default|GetMinutes) (Utilities|Text|ToText(Integer) _output_get_2))))))
    (else
      (bind _result_2 (Math|Integer|IncrementInt (Variables|Default|GetSec))
        (:%20%20
          (bind _output_get_3 (Variables|Default|SetSec _result_2))
          (Rendering|Components|TextRender|SetText (Variables|Default|GetSeconds) (Utilities|Text|ToText(Integer) _output_get_3)))))))

(fn ConstructionScript)