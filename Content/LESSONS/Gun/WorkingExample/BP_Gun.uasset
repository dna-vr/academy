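; A grabbable gun from a lesson example that can be picked up, dropped and fired.
; Pickup stops physics on the mesh, attaches the root to the given component and applies a fixed mesh offset; Drop detaches it and restores physics.
; Both events update the GunHandState flag, which this file never reads.
; Shooting spawns BP_BulletFire at the Arrow component's location, without passing the arrow's rotation.
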(event EventBeginPlay)

(event Collision|EventActorBeginOverlap
  (params (OtherActor :type Actor%20Object%20Reference)))

(event EventTick
  (params (DeltaSeconds :type Float%20%28single-precision%29)))

(event EventPickup
  (params (AttachTo :type Scene%20Component%20Object%20Reference))
  (Variables|Default|SetGunHandState true)
  (Physics|SetSimulatePhysics (Variables|Debug|GetStaticMeshComponent) false)
  (Transformation|AttachComponentToComponent (VehicleSound|GetRootComponent) AttachTo "None" "SnapToTarget" "SnapToTarget" "KeepWorld" false)
  (Transformation|SetRelativeLocationAndRotation (Variables|Debug|GetStaticMeshComponent) "1.000001,-0.999999,6.000000" "0,90.000053, 0" false false))

(event EventDrop
  (Variables|Default|SetGunHandState false)
  (Physics|SetSimulatePhysics (Variables|Debug|GetStaticMeshComponent) true)
  (Transformation|DetachFromActor "KeepWorld" "KeepWorld" "KeepWorld"))

(fn ConstructionScript)

(fn Shooting
  (Game|SpawnActorfromClass "/Game/LESSONS/Gun/WorkingExample/BP_BulletFire.BP_BulletFire_C" (Math|Transform|MakeTransform (Transformation|GetWorldLocation (Variables|Default|GetArrow)) "0, 0, 0" "1,1,1") "Undefined" 0 0))