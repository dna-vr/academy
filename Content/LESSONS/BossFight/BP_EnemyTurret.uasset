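; BP_EnemyTurret is a boss-fight lesson turret that fires laser shots at a player it sees.
; PawnSensing detects the MotionControllerPawn and snaps the actor to face it each time it is seen.
; It then spawns a BP_LaserShooter at ProjectileSpawnLocation and launches its sphere with a velocity-change impulse along the mesh's forward vector.
; A boolean gate with a Delay limits the fire rate.
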(event OnSeePawn(PawnSensing)
  (params (Pawn :type Pawn%20Object%20Reference))
  (bind _asmotion_controller_pawn (Utilities|Casting|CastToMotionControllerPawn Pawn))
  (Utilities|FlowControl|Sequence
    (:then_0
      (Transformation|SetActorRotation (Math|Rotator|FindLookatRotation (Transformation|GetActorLocation) (Transformation|GetActorLocation _asmotion_controller_pawn))))
    (:then_1
      (if (Variables|Default|GetSpawnProjectile)
        (bind _returnvalue (Game|SpawnActorfromClass "/Game/MAIN/BP_LaserShooter.BP_LaserShooter_C" (Transformation|GetWorldTransform (Variables|Default|GetProjectileSpawnLocation)) "Undefined" 0 0))
        (Physics|AddImpulse (Variables|/Game/MAIN/BP_LaserShooter.BP_LaserShooter_C|GetSphere1 _returnvalue) (* (Math|Vector|GetForwardVector (Variables|Default|GetStaticMesh)) (Variables|Default|GetShootForce)) "None" true)
        (Variables|Default|SetSpawnProjectile false)
        (Utilities|FlowControl|Delay 1.5)
        (Variables|Default|SetSpawnProjectile true)))))

(event EventBeginPlay)

(event Collision|EventActorBeginOverlap
  (params (OtherActor :type Actor%20Object%20Reference)))

(event EventTick
  (params (DeltaSeconds :type Float%20%28single-precision%29)))

(fn ConstructionScript)