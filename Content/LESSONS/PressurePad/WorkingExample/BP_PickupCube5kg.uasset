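; BP_PickupCube5kg is a weighted cube for a pressure pad lesson that can be picked up and dropped.
; Actor begin and end overlap events cast to PPad and add or subtract the cube's ItemWeight from the pad's CurrentWeight.
; Pickup, called by BP_MotionController, disables physics and attaches the cube to the given component, while Drop restores physics and detaches it.
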(event EventBeginPlay)

(event Collision|EventActorBeginOverlap
  (params (OtherActor :type Actor%20Object%20Reference))
  ;[1 0.1146 0.5288] PressurePad
  (bind _asppad (Utilities|Casting|CastToPPad OtherActor))
  (Variables|/Game/LESSONS/PressurePad/WorkingExample/PPad.PPad_C|SetCurrentWeight _asppad (+ (Variables|/Game/LESSONS/PressurePad/WorkingExample/PPad.PPad_C|GetCurrentWeight _asppad) (Variables|Default|GetItemWeight))) ; New Weight = \nOld Weight + Item Weight
)

(event EventTick
  (params (DeltaSeconds :type Float%20%28single-precision%29)))

(event EventPickup
  (params (AttachTo :type Scene%20Component%20Object%20Reference))
  (Physics|SetSimulatePhysics (Variables|Debug|GetStaticMeshComponent) false)
  (Transformation|AttachComponentToComponent (VehicleSound|GetRootComponent) AttachTo "None" "KeepWorld" "KeepWorld" "KeepWorld" false))

(event Collision|EventActorEndOverlap
  (params (OtherActor :type Actor%20Object%20Reference))
  ;[1 0.1146 0.5288] PressurePad
  (bind _asppad (Utilities|Casting|CastToPPad OtherActor))
  (Variables|/Game/LESSONS/PressurePad/WorkingExample/PPad.PPad_C|SetCurrentWeight _asppad (- (Variables|/Game/LESSONS/PressurePad/WorkingExample/PPad.PPad_C|GetCurrentWeight _asppad) (Variables|Default|GetItemWeight))) ; New Weight =\nOld Weight - Item Weight
)

(event EventDrop
  (Physics|SetSimulatePhysics (Variables|Debug|GetStaticMeshComponent) true)
  (Transformation|DetachFromActor "KeepWorld" "KeepWorld" "KeepWorld"))

(fn ConstructionScript)