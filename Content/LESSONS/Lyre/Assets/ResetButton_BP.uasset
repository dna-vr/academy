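; ResetButton_BP is a reset button in the Lyre lesson that clears the lyre's recorded notes when a motion controller touches it.
; On BeginPlay it puts a dynamic instance of String_M on its mesh.
; When a BP_MotionController overlaps its Box, it empties the BackupNote and LyreNote arrays on PlayRef and prints a debug message.
; The same hit plays a timeline that drives the material's Glow parameter as visual feedback.
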(event OnComponentBeginOverlap(Box)
  (params (OverlappedComponent :type Primitive%20Component%20Object%20Reference) (OtherActor :type Actor%20Object%20Reference) (OtherComp :type Primitive%20Component%20Object%20Reference) (OtherBodyIndex :type Integer) (bFromSweep :type Boolean) (SweepResult :type Hit%20Result%20Structure%20%28by%20ref%29))
  (bind _playref (Variables|Default|GetPlayRef))
  (Utilities|Casting|CastToBP_MotionController OtherActor)
  (Utilities|FlowControl|Sequence
    (:then_0
      (Development|PrintString "RESET BUTTON HIT")
      (Utilities|Array|Clear (Variables|/Game/LESSONS/Lyre/Assets/PlayButton_BP.PlayButton_BP_C|GetBackup_Note _playref))
      (Utilities|Array|Clear (Variables|/Game/LESSONS/Lyre/Assets/PlayButton_BP.PlayButton_BP_C|GetLyre_Note _playref)))
    (:then_1
      (bind _newtrack_2 (Timeline|Timeline_0 PlayFromStart)
        (:Update
          (Rendering|Material|SetScalarParameterValue (stale EventBeginPlay _returnvalue) "Glow" _newtrack_2 :!class /Script/Engine.MaterialInstanceDynamic))))))

(event EventBeginPlay
  (bind _staticmesh (Variables|Default|GetStaticMesh))
  (bind _returnvalue (Rendering|Material|CreateDynamicMaterialInstance _staticmesh 0 "/Game/LESSONS/Lyre/Assets/String_M.String_M" "None" :!class /Script/Engine.PrimitiveComponent))
  (Rendering|Material|SetMaterial _staticmesh 0 _returnvalue))

(event Collision|EventActorBeginOverlap
  (params (OtherActor :type Actor%20Object%20Reference)))

(event EventTick
  (params (DeltaSeconds :type Float%20%28single-precision%29)))

(fn ConstructionScript)