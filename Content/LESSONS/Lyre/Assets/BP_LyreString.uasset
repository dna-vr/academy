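; BP_LyreString is a VR lyre string that plays its note and glows when a motion controller touches it.
; A capsule overlap with BP_MotionController plays LyreNote as 2D sound and restarts the Glowing timeline, which drives the Glow parameter on a dynamic material created at BeginPlay.
; When the timeline finishes, the string appends its note to PlayButton's NoteSequencePlayed array, recording the played sequence.
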(event OnComponentBeginOverlap(Capsule)
  (params (OverlappedComponent :type Primitive%20Component%20Object%20Reference) (OtherActor :type Actor%20Object%20Reference) (OtherComp :type Primitive%20Component%20Object%20Reference) (OtherBodyIndex :type Integer) (bFromSweep :type Boolean) (SweepResult :type Hit%20Result%20Structure%20%28by%20ref%29))
  (bind _lyre_note (Variables|Default|GetLyre_Note))
  (Utilities|Casting|CastToBP_MotionController OtherActor)
  (Audio|PlaySound2D _lyre_note 1.0 1.0 0.0 0 0)
  (bind _newtrack_0 (Timeline|Glowing PlayFromStart)
    (:Update
      (Rendering|Material|SetScalarParameterValue (stale EventBeginPlay _returnvalue) "Glow" _newtrack_0 :!class /Script/Engine.MaterialInstanceDynamic))
    (:Finished
      (Utilities|Array|Add (Variables|/Game/LESSONS/Lyre/Assets/BP_Play.BP_Play_C|GetNoteSequencePlayed (Variables|Default|GetPlayButton)) _lyre_note))))

(event EventBeginPlay
  (bind _staticmesh (Variables|Default|GetStaticMesh))
  (bind _returnvalue (Rendering|Material|CreateDynamicMaterialInstance _staticmesh 0 "/Game/LESSONS/Lyre/Assets/String_M.String_M" "None" :!class /Script/Engine.PrimitiveComponent))
  (Rendering|Material|SetMaterial _staticmesh 0 _returnvalue))

(event Collision|EventActorBeginOverlap
  (params (OtherActor :type Actor%20Object%20Reference)))

(fn ConstructionScript)