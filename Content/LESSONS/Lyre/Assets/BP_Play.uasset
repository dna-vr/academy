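; BP_Play is a touch-triggered object in the lyre lesson that plays a preset note pattern when a BP_MotionController overlaps its box.
; A DoOnce with a delayed reset prevents the pattern sound from retriggering during playback.
; Each overlap also restarts a timeline that drives the Glow parameter on a dynamic string material created at BeginPlay.
; Tick trims NoteSequencePlayed to five entries, though nothing here fills or reads that array otherwise.
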(event OnComponentBeginOverlap(Box)
  (params (OverlappedComponent :type Primitive%20Component%20Object%20Reference) (OtherActor :type Actor%20Object%20Reference) (OtherComp :type Primitive%20Component%20Object%20Reference) (OtherBodyIndex :type Integer) (bFromSweep :type Boolean) (SweepResult :type Hit%20Result%20Structure%20%28by%20ref%29))
  (Utilities|Casting|CastToBP_MotionController OtherActor)
  (Utilities|FlowControl|Sequence
    (:then_0
      (Utilities|FlowControl|DoOnce false :!label _label
        (:Completed
          (Audio|PlaySound2D "/Game/LESSONS/Lyre/Assets/SFX/Lyre_Pattern_12135.Lyre_Pattern_12135" 1.0 1.0 0.0 0 0) ; play win sequence
          (Utilities|FlowControl|Delay 3.0)
          (goto _label Reset))))
    (:then_1
      (bind _newtrack_2 (Timeline|Timeline_0 PlayFromStart)
        (:Update
          (Rendering|Material|SetScalarParameterValue (stale EventBeginPlay _returnvalue) "Glow" _newtrack_2 :!class /Script/Engine.MaterialInstanceDynamic))))))

(event EventBeginPlay
  (bind _staticmesh (Variables|Default|GetStaticMesh))
  (bind _returnvalue (Rendering|Material|CreateDynamicMaterialInstance _staticmesh 0 "/Game/LESSONS/Lyre/Assets/String_M.String_M" "None" :!class /Script/Engine.PrimitiveComponent))
  (Rendering|Material|SetMaterial _staticmesh 0 _returnvalue))

(event EventTick
  (params (DeltaSeconds :type Float%20%28single-precision%29))
  (bind _notesequenceplayed (Variables|Default|GetNoteSequencePlayed))
  ;[1 1 1] remove first note if there are more than 5 played
  (if (> (Utilities|Array|Length _notesequenceplayed) 5)
    (Utilities|Array|RemoveIndex _notesequenceplayed)))

(fn ConstructionScript)