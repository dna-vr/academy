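; BP_Torch_Off is a torch for the fire puzzle that starts unlit and can be picked up by a motion controller.
; BeginPlay hides the particle system and point light, clears FireState, and binds handlers to the TurnOnFire and TurnOffFire dispatchers that toggle their visibility.
; Pickup disables mesh physics and attaches the root to the supplied component, while Drop re-enables physics and detaches the actor.
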(event Custom|TurnOnFire_Event_0
  (Rendering|SetVisibility (Variables|Default|GetParticleSystem) true false))

(event Custom|TurnOffFire_Event_0
  (Rendering|SetVisibility (Variables|Default|GetParticleSystem) false false))

(event EventBeginPlay
  ;[1 0.02083 0.02083] Turn off fire by default
  (Rendering|SetVisibility (Variables|Default|GetParticleSystem) false false)
  (Variables|Default|SetFireState false)
  (EventDispatchers|AssignTurnonFire (delegate Custom|TurnOnFire_Event_0))
  (EventDispatchers|AssignTurnOffFire (delegate Custom|TurnOffFire_Event_0)))

(event EventPickup
  (params (AttachTo :type Scene%20Component%20Object%20Reference))
  (Physics|SetSimulatePhysics (Variables|Debug|GetStaticMeshComponent) false)
  (Transformation|AttachComponentToComponent (VehicleSound|GetRootComponent) AttachTo "None" "KeepWorld" "KeepWorld" "KeepWorld" false))

(event EventDrop
  (Physics|SetSimulatePhysics (Variables|Debug|GetStaticMeshComponent) true)
  (Transformation|DetachFromActor "KeepWorld" "KeepWorld" "KeepWorld"))

(fn ConstructionScript)